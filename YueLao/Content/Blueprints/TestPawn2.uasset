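; Player 2 pawn that moves on gamepad D-pad input and loses health as it travels.
; Each direction uses gates and flip-flops to start or stop a timeline that sets animation speed and offsets location.
; Each movement update subtracts Displacement from health, updating the UMG bar; once depleted, Died ragdolls the mesh on movement input.
; When both players are dead, LoseScreen waits, then opens the level-specific loss map.
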(event `LoseScreen`
  (`KismetSystemLibrary.Delay` 2.0)
  (bind _returnvalue (`GameplayStatics.GetCurrentLevelName` true))
  (if (`KismetStringLibrary.EqualEqual_StrStr` _returnvalue "Level01")
    (`GameplayStatics.OpenLevel` "YouLost01")
    (else
      (`GameplayStatics.OpenLevel` "YouLost02"))))

(event `Key|Gamepad_DPad_Right`
  (params (Key :type "Key Structure"))
  (bind (_returnvalue_x _returnvalue_y _returnvalue_z) (`KismetMathLibrary.BreakVector` (`self.K2_GetActorLocation`)))
  (:`Pressed`
    (`|ExecutionSequence`
      (:`then_0`
        (goto _label :!via `Open`))
      (:`then_1`
        (`/Engine/EditorBlueprintResources/StandardMacros.Gate` true :!label _label
          (:`Exit`
            (if (`self.Player2Died`)
              (`self.Died`)
              (bind (_direction _newtrack_0) (`Timeline|Timeline_0` :!via `Stop` :!label _label_2)
                (:`Update`
                  (set `self.AnimSpeed` _newtrack_0)
                  (`self.K2_SetActorLocation` (`KismetMathLibrary.MakeVector` (+ _returnvalue_x (`self.Displacement`)) _returnvalue_y _returnvalue_z))
                  (`self.SetHealthPercentP2` :!label _label_3)))
              (else
                (bind _isa (`/Engine/EditorBlueprintResources/StandardMacros.FlipFlop`)
                  (:`A`
                    _)
                  (:`B`
                    _))
                (if _isa
                  (`AudioComponent.Play` (`self.Player_Move_RGT`) 0.0)
                  (`SceneComponent.K2_SetWorldRotation` (`self.SkeletalMesh`) (struct :`Yaw` -90.0) false false)
                  (goto _label_2)
                  (else
                    (set `self.AnimSpeed` 187.5)
                    (goto _label_2 :!via `Stop`))))))))))
  (:`Released`
    (`|ExecutionSequence`
      (:`then_0`
        (goto _label))
      (:`then_1`
        (`/Engine/EditorBlueprintResources/StandardMacros.DoOnce` false
          (:`Completed`
            (goto _label :!via `Toggle`)))))))

(event `Key|Gamepad_DPad_Left`
  (params (Key :type "Key Structure"))
  (bind (_returnvalue_x _returnvalue_y _returnvalue_z) (`KismetMathLibrary.BreakVector` (`self.K2_GetActorLocation`)))
  (:`Pressed`
    (`|ExecutionSequence`
      (:`then_0`
        (goto _label_4 :!via `Open`))
      (:`then_1`
        (`/Engine/EditorBlueprintResources/StandardMacros.Gate` true :!label _label_4
          (:`Exit`
            (if (`self.Player2Died`)
              (`self.Died`)
              (bind (_direction _newtrack_0) (`Timeline|Timeline_1` :!via `Stop` :!label _label_5)
                (:`Update`
                  (set `self.AnimSpeed` _newtrack_0)
                  (`self.K2_SetActorLocation` (`KismetMathLibrary.MakeVector` (+ _returnvalue_x (* (`self.Displacement`) -1.0)) _returnvalue_y _returnvalue_z))
                  (goto _label_3)))
              (else
                (bind _isa (`/Engine/EditorBlueprintResources/StandardMacros.FlipFlop`)
                  (:`A`
                    _)
                  (:`B`
                    _))
                (if _isa
                  (`AudioComponent.Play` (`self.Player_MoveLFT`) 0.0)
                  (`SceneComponent.K2_SetWorldRotation` (`self.SkeletalMesh`) (struct :`Yaw` 90.0) false false)
                  (goto _label_5)
                  (else
                    (set `self.AnimSpeed` 187.5)
                    (goto _label_5 :!via `Stop`))))))))))
  (:`Released`
    (`|ExecutionSequence`
      (:`then_0`
        (goto _label_4))
      (:`then_1`
        (`/Engine/EditorBlueprintResources/StandardMacros.DoOnce` false
          (:`Completed`
            (goto _label_4 :!via `Toggle`)))))))

(event `Key|Gamepad_DPad_Up`
  (params (Key :type "Key Structure"))
  (bind (_returnvalue_x _returnvalue_y _returnvalue_z) (`KismetMathLibrary.BreakVector` (`self.K2_GetActorLocation`)))
  (:`Pressed`
    (`|ExecutionSequence`
      (:`then_0`
        (goto _label_6 :!via `Open`))
      (:`then_1`
        (`/Engine/EditorBlueprintResources/StandardMacros.Gate` true :!label _label_6
          (:`Exit`
            (if (`self.Player2Died`)
              (`self.Died`)
              (bind (_direction _newtrack_0) (`Timeline|Timeline_2` :!via `Stop` :!label _label_7)
                (:`Update`
                  (set `self.AnimSpeed` _newtrack_0)
                  (`self.K2_SetActorLocation` (`KismetMathLibrary.MakeVector` _returnvalue_x (+ _returnvalue_y (* (`self.Displacement`) -1.0)) _returnvalue_z))
                  (goto _label_3)))
              (else
                (bind _isa (`/Engine/EditorBlueprintResources/StandardMacros.FlipFlop`)
                  (:`A`
                    _)
                  (:`B`
                    _))
                (if _isa
                  (`AudioComponent.Play` (`self.Player_Move_FWD`) 0.0)
                  (`SceneComponent.K2_SetWorldRotation` (`self.SkeletalMesh`) (struct :`Yaw` 180.0) false false)
                  (goto _label_7)
                  (else
                    (set `self.AnimSpeed` 187.5)
                    (goto _label_7 :!via `Stop`))))))))))
  (:`Released`
    (`|ExecutionSequence`
      (:`then_0`
        (goto _label_6))
      (:`then_1`
        (`/Engine/EditorBlueprintResources/StandardMacros.DoOnce` false
          (:`Completed`
            (goto _label_6 :!via `Toggle`)))))))

(event `Key|Gamepad_DPad_Down`
  (params (Key :type "Key Structure"))
  (bind (_returnvalue_x _returnvalue_y _returnvalue_z) (`KismetMathLibrary.BreakVector` (`self.K2_GetActorLocation`)))
  (:`Pressed`
    (`|ExecutionSequence`
      (:`then_0`
        (goto _label_8 :!via `Open`))
      (:`then_1`
        (`/Engine/EditorBlueprintResources/StandardMacros.Gate` true :!label _label_8
          (:`Exit`
            (if (`self.Player2Died`)
              (`self.Died`)
              (bind (_direction _newtrack_0) (`Timeline|Timeline_3` :!via `Stop` :!label _label_9)
                (:`Update`
                  (set `self.AnimSpeed` _newtrack_0)
                  (`self.K2_SetActorLocation` (`KismetMathLibrary.MakeVector` _returnvalue_x (+ _returnvalue_y (`self.Displacement`)) _returnvalue_z))
                  (goto _label_3)))
              (else
                (bind _isa (`/Engine/EditorBlueprintResources/StandardMacros.FlipFlop`)
                  (:`A`
                    _)
                  (:`B`
                    _))
                (if _isa
                  (`AudioComponent.Play` (`self.Player_Move_BWD`) 0.0)
                  (`SceneComponent.K2_SetWorldRotation` :`self` (`self.SkeletalMesh`))
                  (goto _label_9)
                  (else
                    (set `self.AnimSpeed` 187.5)
                    (goto _label_9 :!via `Stop`))))))))))
  (:`Released`
    (`|ExecutionSequence`
      (:`then_0`
        (goto _label_8))
      (:`then_1`
        (`/Engine/EditorBlueprintResources/StandardMacros.DoOnce` false
          (:`Completed`
            (goto _label_8 :!via `Toggle`)))))))

(fn `CheckDead`
  (if (and (`self.Player2Died`) (`/Game/Blueprints/TestPawn1.Player1Dead` (`self.Player1`)))
    (`self.LoseScreen`)))

(fn `Died`
  (bind _skeletalmesh (`self.SkeletalMesh`))
  (`PrimitiveComponent.SetCollisionEnabled` (`self.Capsule`) "NoCollision")
  (`PrimitiveComponent.SetSimulatePhysics` _skeletalmesh true)
  (`PrimitiveComponent.SetCollisionEnabled` _skeletalmesh "QueryAndPhysics")
  (`SkeletalMeshComponent.SetAnimationMode` _skeletalmesh "AnimationCustomMode"))

(fn `SetHealthPercentP2`
  (bind _returnvalue (- (`self.CurrentHealth`) (`self.Displacement`)))
  (set `self.CurrentHealth` _returnvalue)
  (`ProgressBar.SetPercent` (`/Game/UMG/UMG_Fatigue.ProgressBar_P2` (`self.UMG`)) (/ _returnvalue (`self.InitialHealth`)))
  (if (<= (`self.CurrentHealth`) 0.0)
    (set `self.Player2Died` true)
    (`self.CheckDead`)))

(fn `UserConstructionScript`)