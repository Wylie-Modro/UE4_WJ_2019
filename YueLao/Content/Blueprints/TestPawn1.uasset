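; Player 1 pawn, tied by a collidable cable to TestPawn2 and sharing a fatigue widget with it.
; WASD toggles per-direction timelines through gates and flip-flops, rotating the mesh and moving the actor along X or Y.
; Each movement update drains health and updates the fatigue bar; once health is empty, movement input triggers ragdoll.
; If TestPawn2 is also dead when checked, a level-specific lose map opens after a delay.
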(event `self.ReceiveBeginPlay`
  (bind _cablerope (`self.CableRope`))
  (set `CableComponent.bEnableCollision` true (`CableActor.CableComponent` (`self.CableRope`)))
  (`self.K2_AttachToComponent` (`self.CableRope`) (`self.Capsule`) "None" "SnapToTarget" "SnapToTarget" "KeepRelative" true)
  (set `CableComponent.EndLocation` (0.0 0.0 0.0) (`CableActor.CableComponent` _cablerope))
  (`CableComponent.SetAttachEndTo` (`CableActor.CableComponent` _cablerope) (`self.TestPawn2`) "None" "None")
  (bind _returnvalue (`|CreateWidget` "/Game/UMG/UMG_Fatigue.UMG_Fatigue_C"))
  (bind _output_get (set `self.UMG_Fatigue` _returnvalue))
  (bind _output_get_2 (set `/Game/Blueprints/TestPawn2.UMG` _output_get (`self.TestPawn2`)))
  (`UserWidget.AddToViewport` _output_get_2 0))

(event `LoseScreen`
  (`KismetSystemLibrary.Delay` 2.0)
  (bind _returnvalue (`GameplayStatics.GetCurrentLevelName` true))
  (if (`KismetStringLibrary.EqualEqual_StrStr` _returnvalue "Level01")
    (`GameplayStatics.OpenLevel` "YouLost1")
    (else
      (`GameplayStatics.OpenLevel` "YouLost2"))))

(event `Key|D`
  (params (Key :type "Key Structure"))
  (bind (_returnvalue_x _returnvalue_y _returnvalue_z) (`KismetMathLibrary.BreakVector` (`self.K2_GetActorLocation`)))
  (:`Pressed`
    (`|ExecutionSequence`
      (:`then_0`
        (goto _label :!via `Open`))
      (:`then_1`
        (`/Engine/EditorBlueprintResources/StandardMacros.Gate` true :!label _label
          (:`Exit`
            (if (`self.Player1Dead`)
              (`self.Died`)
              (bind (_direction _newtrack_0) (`Timeline|Timeline_0` :!via `Stop` :!label _label_2)
                (:`Update`
                  (set `self.AnimSpeed` _newtrack_0)
                  (`self.K2_SetActorLocation` (`KismetMathLibrary.MakeVector` (+ _returnvalue_x (`self.Displacement`)) _returnvalue_y _returnvalue_z))
                  (`self.SetHealthPercentP1` :!label _label_3)))
              (else
                (bind _isa (`/Engine/EditorBlueprintResources/StandardMacros.FlipFlop`)
                  (:`A`
                    _)
                  (:`B`
                    _))
                (if _isa
                  (`AudioComponent.Play` (`self.Player_Move_RGT`) 0.0)
                  (`SceneComponent.K2_SetWorldRotation` (`self.SkeletalMesh`) (struct :`Yaw` -90.0) false false)
                  (goto _label_2)
                  (else
                    (set `self.AnimSpeed` 187.5)
                    (goto _label_2 :!via `Stop`))))))))))
  (:`Released`
    (`|ExecutionSequence`
      (:`then_0`
        (goto _label))
      (:`then_1`
        (`/Engine/EditorBlueprintResources/StandardMacros.DoOnce` false
          (:`Completed`
            (goto _label :!via `Toggle`)))))))

(event `Key|A`
  (params (Key :type "Key Structure"))
  (bind (_returnvalue_x _returnvalue_y _returnvalue_z) (`KismetMathLibrary.BreakVector` (`self.K2_GetActorLocation`)))
  (:`Pressed`
    (`|ExecutionSequence`
      (:`then_0`
        (goto _label_4 :!via `Open`))
      (:`then_1`
        (`/Engine/EditorBlueprintResources/StandardMacros.Gate` true :!label _label_4
          (:`Exit`
            (if (`self.Player1Dead`)
              (`self.Died`)
              (bind (_direction _newtrack_0) (`Timeline|Timeline_1` :!via `Stop` :!label _label_5)
                (:`Update`
                  (set `self.AnimSpeed` _newtrack_0)
                  (`self.K2_SetActorLocation` (`KismetMathLibrary.MakeVector` (+ _returnvalue_x (* (`self.Displacement`) -1.0)) _returnvalue_y _returnvalue_z))
                  (goto _label_3)))
              (else
                (bind _isa (`/Engine/EditorBlueprintResources/StandardMacros.FlipFlop`)
                  (:`A`
                    _)
                  (:`B`
                    _))
                (if _isa
                  (`AudioComponent.Play` (`self.Player_MoveLFT`) 0.0)
                  (`SceneComponent.K2_SetWorldRotation` (`self.SkeletalMesh`) (struct :`Yaw` 90.0) false false)
                  (goto _label_5)
                  (else
                    (set `self.AnimSpeed` 187.5)
                    (goto _label_5 :!via `Stop`))))))))))
  (:`Released`
    (`|ExecutionSequence`
      (:`then_0`
        (goto _label_4))
      (:`then_1`
        (`/Engine/EditorBlueprintResources/StandardMacros.DoOnce` false
          (:`Completed`
            (goto _label_4 :!via `Toggle`)))))))

(event `Key|W`
  (params (Key :type "Key Structure"))
  (bind (_returnvalue_x _returnvalue_y _returnvalue_z) (`KismetMathLibrary.BreakVector` (`self.K2_GetActorLocation`)))
  (:`Pressed`
    (`|ExecutionSequence`
      (:`then_0`
        (goto _label_6 :!via `Open`))
      (:`then_1`
        (`/Engine/EditorBlueprintResources/StandardMacros.Gate` true :!label _label_6
          (:`Exit`
            (if (`self.Player1Dead`)
              (`self.Died`)
              (bind (_direction _newtrack_0) (`Timeline|Timeline_2` :!via `Stop` :!label _label_7)
                (:`Update`
                  (set `self.AnimSpeed` _newtrack_0)
                  (`self.K2_SetActorLocation` (`KismetMathLibrary.MakeVector` _returnvalue_x (+ _returnvalue_y (* (`self.Displacement`) -1.0)) _returnvalue_z))
                  (goto _label_3)))
              (else
                (bind _isa (`/Engine/EditorBlueprintResources/StandardMacros.FlipFlop`)
                  (:`A`
                    _)
                  (:`B`
                    _))
                (if _isa
                  (`AudioComponent.Play` (`self.Player_Move_FWD`) 0.0)
                  (`SceneComponent.K2_SetWorldRotation` (`self.SkeletalMesh`) (struct :`Yaw` 180.0) false false)
                  (goto _label_7)
                  (else
                    (set `self.AnimSpeed` 187.5)
                    (goto _label_7 :!via `Stop`))))))))))
  (:`Released`
    (`|ExecutionSequence`
      (:`then_0`
        (goto _label_6))
      (:`then_1`
        (`/Engine/EditorBlueprintResources/StandardMacros.DoOnce` false
          (:`Completed`
            (goto _label_6 :!via `Toggle`)))))))

(event `Key|S`
  (params (Key :type "Key Structure"))
  (bind (_returnvalue_x _returnvalue_y _returnvalue_z) (`KismetMathLibrary.BreakVector` (`self.K2_GetActorLocation`)))
  (:`Pressed`
    (`|ExecutionSequence`
      (:`then_0`
        (goto _label_8 :!via `Open`))
      (:`then_1`
        (`/Engine/EditorBlueprintResources/StandardMacros.Gate` true :!label _label_8
          (:`Exit`
            (if (`self.Player1Dead`)
              (`self.Died`)
              (bind (_direction _newtrack_0) (`Timeline|Timeline_3` :!via `Stop` :!label _label_9)
                (:`Update`
                  (set `self.AnimSpeed` _newtrack_0)
                  (`self.K2_SetActorLocation` (`KismetMathLibrary.MakeVector` _returnvalue_x (+ _returnvalue_y (`self.Displacement`)) _returnvalue_z))
                  (goto _label_3)))
              (else
                (bind _isa (`/Engine/EditorBlueprintResources/StandardMacros.FlipFlop`)
                  (:`A`
                    _)
                  (:`B`
                    _))
                (if _isa
                  (`AudioComponent.Play` (`self.Player_Move_BWD`) 0.0)
                  (`SceneComponent.K2_SetWorldRotation` :`self` (`self.SkeletalMesh`))
                  (goto _label_9)
                  (else
                    (set `self.AnimSpeed` 187.5)
                    (goto _label_9 :!via `Stop`))))))))))
  (:`Released`
    (`|ExecutionSequence`
      (:`then_0`
        (goto _label_8))
      (:`then_1`
        (`/Engine/EditorBlueprintResources/StandardMacros.DoOnce` false
          (:`Completed`
            (goto _label_8 :!via `Toggle`)))))))

(fn `CheckDead`
  (if (and (`self.Player1Dead`) (`/Game/Blueprints/TestPawn2.Player2Died` (`self.TestPawn2`)))
    (`self.LoseScreen`)))

(fn `Died`
  (bind _skeletalmesh (`self.SkeletalMesh`))
  (`PrimitiveComponent.SetCollisionEnabled` (`self.Capsule`) "NoCollision")
  (`PrimitiveComponent.SetSimulatePhysics` _skeletalmesh true)
  (`PrimitiveComponent.SetCollisionEnabled` _skeletalmesh "QueryAndPhysics")
  (`SkeletalMeshComponent.SetAnimationMode` _skeletalmesh "AnimationCustomMode"))

(fn `SetHealthPercentP1`
  (bind _returnvalue (- (`self.CurrentHealth`) (`self.Displacement`)))
  (set `self.CurrentHealth` _returnvalue)
  (`ProgressBar.SetPercent` (`/Game/UMG/UMG_Fatigue.ProgressBar_P1` (`self.UMG_Fatigue`)) (/ _returnvalue (`self.InitialHealth`)))
  (if (<= (`self.CurrentHealth`) 0.0)
    (set `self.Player1Dead` true)
    (`self.CheckDead`)))

(fn `UserConstructionScript`)