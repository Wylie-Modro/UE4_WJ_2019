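; CableRope is a Blueprint that makes static mesh components follow the particles of a cable component.
; BeginPlay adds one scaled-down mesh per cable particle location and stores them in the Squares array.
; Tick moves each stored mesh to its particle's current world location by array index, without sweeping.
; An unconnected node would join two TestPawn capsules with a physics constraint, but it never runs.
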(event `self.ReceiveBeginPlay`
  (for _array_element (`CableComponent.GetCableParticleLocations` (`self.CableComponent`))
    (bind _returnvalue (`AddComponent|NODE_AddStaticMeshComponent-0` :`RelativeTransform` (`KismetMathLibrary.MakeTransform` _array_element (struct) (0.1 0.1 0.1))))
    (`KismetArrayLibrary.Array_Add` (`self.Squares`) _returnvalue)))

(event `self.ReceiveTick`
  (params (DeltaSeconds :type "Float (single-precision)"))
  (for (_array_element _array_index) (`CableComponent.GetCableParticleLocations` (`self.CableComponent`))
    (`SceneComponent.K2_SetWorldLocation` (`|GetArrayItem` (`self.Squares`) _array_index) _array_element false false)))

(fn `UserConstructionScript`)